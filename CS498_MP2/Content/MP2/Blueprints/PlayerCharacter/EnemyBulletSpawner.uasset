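; Enemy turret actor that shoots EnemyBullet at the learning-kit player character while the player's mesh overlaps its AttackRange.
; Tick feeds a one-second Delay that throttles firing, then turns the actor toward the player and spawns a bullet from the Cone.
; Shots lead the target by offsetting the aim with player velocity scaled by distance.
; The turret is destroyed when the player enters DeathBox or a Bullet hits ShootBox.
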(event `self.ReceiveBeginPlay`
  (`self.EnableInput` (`GameplayStatics.GetPlayerController` 0))
  (bind _asbp_learning_kit_player_character (cast `/Game/MP2/Blueprints/PlayerCharacter/BP_LearningKit_PlayerCharacter` (`GameplayStatics.GetPlayerPawn` 0)))
  (set `self.PlayerRef` _asbp_learning_kit_player_character))

(event `self.ReceiveTick`
  (params (DeltaSeconds :type "Float (single-precision)"))
  (bind _playerref (`self.PlayerRef`))
  (bind _returnvalue (`SceneComponent.K2_GetComponentLocation` (`self.Cone`)))
  (bind _returnvalue_2 (`SceneComponent.K2_GetComponentLocation` (`Character.Mesh` _playerref)))
  (bind _asbp_learning_kit_player_character (cast `/Game/MP2/Blueprints/PlayerCharacter/BP_LearningKit_PlayerCharacter` (`GameplayStatics.GetPlayerPawn` 0)))
  (if (`PrimitiveComponent.IsOverlappingComponent` (`self.attack range`) (`Character.Mesh` _asbp_learning_kit_player_character))
    (`KismetSystemLibrary.Delay` 1.0)
    (`self.K2_SetActorRotation` (`KismetMathLibrary.FindLookAtRotation` _returnvalue _returnvalue_2))
    (`|SpawnActorFromClass` "/Game/MP2/Blueprints/PlayerCharacter/EnemyBullet.EnemyBullet_C" (`KismetMathLibrary.MakeTransform` _returnvalue (`KismetMathLibrary.FindLookAtRotation` _returnvalue (+ _returnvalue_2 (* (`self.GetVelocity` _playerref) (/ (`self.GetDistanceTo` _playerref) 1500.0))))) "Undefined" "OverrideRootScale" null null)))

(event `self.DeathBox.OnComponentBeginOverlap`
  (params (OverlappedComponent :type "PrimitiveComponent Object Reference") (OtherActor :type "Actor Object Reference") (OtherComp :type "PrimitiveComponent Object Reference") (OtherBodyIndex :type Integer) (bFromSweep :type Boolean) (SweepResult :type "HitResult Structure (by ref)"))
  (cast `/Game/MP2/Blueprints/PlayerCharacter/BP_LearningKit_PlayerCharacter` OtherActor)
  (`self.K2_DestroyActor`))

(event `self.ShootBox.OnComponentBeginOverlap`
  (params (OverlappedComponent :type "PrimitiveComponent Object Reference") (OtherActor :type "Actor Object Reference") (OtherComp :type "PrimitiveComponent Object Reference") (OtherBodyIndex :type Integer) (bFromSweep :type Boolean) (SweepResult :type "HitResult Structure (by ref)"))
  (cast `/Game/MP2/Blueprints/PlayerCharacter/Bullet` OtherActor)
  (`self.K2_DestroyActor`))

(fn `UserConstructionScript`)